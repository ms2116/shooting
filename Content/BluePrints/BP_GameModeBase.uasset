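; Game mode Blueprint that tracks the current score and a persistent best score.
; On BeginPlay it adds WBP_MainWidget to the viewport, then loads BestScore from the "BestScoreData" save slot if one exists.
; AddScore accumulates points and, whenever the total beats BestScore, immediately saves it through a newly created BP_SaveScore object.
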(event EventBeginPlay
  (bind _returnvalue (UserInterface|CreateWidget "/Game/UI/WBP_MainWidget.WBP_MainWidget_C"))
  (UserInterface|Viewport|AddtoViewport _returnvalue 0)
  (bind _bestscore (CallFunction|LoadScoreData))
  (Variables|Default|SetBestScore _bestscore))

(event EventTick
  (params (DeltaSeconds :type Float%20%28single-precision%29)))

(fn ConstructionScript)

(fn AddScore
  (params (Point :type Integer))
  (Variables|Default|SetCurrentScore (+ Point (Variables|Default|GetCurrentScore)))
  (if (> (Variables|Default|GetCurrentScore) (Variables|Default|GetBestScore))
    (bind _output_get (Variables|Default|SetBestScore (Variables|Default|GetCurrentScore)))
    (CallFunction|SaveScoreData _output_get)))

(fn SaveScoreData
  (params (SaveValue :type Integer))
  (bind _returnvalue (SaveGame|CreateSaveGameObject "/Game/BluePrints/BP_SaveScore.BP_SaveScore_C"))
  (bind _output_get (Variables|Default|SetSaveInstance _returnvalue))
  (Variables|/Game/BluePrints/BP_SaveScore.BP_SaveScore_C|SetScoreData _output_get SaveValue)
  (SaveGame|SaveGametoSlot _output_get "BestScoreData"))

(fn LoadScoreData
  (bind _returnvalue (SaveGame|DoesSaveGameExist "BestScoreData"))
  (if _returnvalue
    (bind _returnvalue_2 (SaveGame|LoadGamefromSlot "BestScoreData"))
    (bind _asbp_save_score (Utilities|Casting|CastToBP_SaveScore _returnvalue_2))
    (return (Variables|/Game/BluePrints/BP_SaveScore.BP_SaveScore_C|GetScoreData _asbp_save_score))))