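; BP_Player is the player actor, which moves in the Y-Z plane and fires projectiles.
; BeginPlay adds the Enhanced Input mapping context, and the horizontal and vertical actions store axis values.
; Tick normalizes those axes and moves the actor by speed and delta time, without sweeping for collisions.
; The fire action waits briefly, then spawns BP_Bullet at the FirePosition component and plays a blaster sound.
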(event Input|EnhancedActionEvents|EnhancedInputActionIA_Fire
  (params (ActionValue :type Boolean) (ElapsedSeconds :type Float%20%28double-precision%29) (TriggeredSeconds :type Float%20%28double-precision%29) (InputAction :type Input%20Action%20Object%20Reference :default "/Game/Inputs/IA_Fire.IA_Fire"))
  (Utilities|FlowControl|Delay 0.1)
  (Game|SpawnActorfromClass "/Game/BluePrints/BP_Bullet.BP_Bullet_C" (Transformation|GetWorldTransform (Variables|Default|GetFire%20Position)) "AlwaysSpawn" "MultiplyWithRoot" 0 0)
  (Audio|PlaySound2D "/Game/Audio/star-wars-blaster.star-wars-blaster" 1.0 1.0 0.0 0 0))

(event Input|EnhancedActionEvents|EnhancedInputActionIA_Horizontal
  (params (ActionValue :type Float%20%28double-precision%29) (ElapsedSeconds :type Float%20%28double-precision%29) (TriggeredSeconds :type Float%20%28double-precision%29) (InputAction :type Input%20Action%20Object%20Reference :default "/Game/Inputs/IA_Horizontal.IA_Horizontal"))
  (:Triggered
    (Variables|Default|SetHorizontal ActionValue :!label _label))
  (:Completed
    (goto _label)))

(event Input|EnhancedActionEvents|EnhancedInputActionIA_Vertical
  (params (ActionValue :type Float%20%28double-precision%29) (ElapsedSeconds :type Float%20%28double-precision%29) (TriggeredSeconds :type Float%20%28double-precision%29) (InputAction :type Input%20Action%20Object%20Reference :default "/Game/Inputs/IA_Vertical.IA_Vertical"))
  (:Triggered
    (Variables|Default|SetVertical ActionValue :!label _label))
  (:Completed
    (goto _label)))

(event EventBeginPlay
  (Input|AddMappingContext (PlayerController|LocalPlayerSubsystems|GetEnhancedInputLocalPlayerSubsystem (Game|GetPlayerController 0)) "/Game/Inputs/IMC_PlayerInput.IMC_PlayerInput" 0 "(bIgnoreAllPressedKeysUntilRelease=True,bForceImmediately=False,bNotifyUserSettings=False)"))

(event Collision|EventActorBeginOverlap
  (params (OtherActor :type Actor%20Object%20Reference)))

(event EventTick
  (params (DeltaSeconds :type Float%20%28single-precision%29))
  (bind _returnvalue (Transformation|SetActorLocation (+ (Transformation|GetActorLocation) (* (* (Math|Vector|Normalize (Math|Vector|MakeVector 0.0 (Variables|Default|GetHorizontal) (Variables|Default|GetVertical))) (Variables|Default|GetMoveSpeed)) DeltaSeconds)) false false)))

(fn ConstructionScript)